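; Base projectile that deals hit-location-based damage between player characters through the Gameplay Ability System, with lifespan set to InitialSpeed / Range.
; On a server-side capsule overlap, a sphere trace toward the victim finds the struck bone.
; Head/neck, torso/upper-arm or other bones select randomized Damage multipliers, passed by SetByCaller into GE_Damaging.
; It then plays a montage on the victim and destroys itself; remote overlaps just destroy it.
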(event `self.ReceiveBeginPlay`
  (set `self.ProjectileOwner` (`self.GetOwner`))
  (`self.SetLifeSpan` (/ (`self.Initial Speed`) (`self.Range`))))

(event `self.Capsule.OnComponentBeginOverlap`
  (params (OverlappedComponent :type "PrimitiveComponent Object Reference") (OtherActor :type "Actor Object Reference") (OtherComp :type "PrimitiveComponent Object Reference") (OtherBodyIndex :type Integer) (bFromSweep :type Boolean) (SweepResult :type "HitResult Structure (by ref)"))
  (bind _returnvalue (* (`self.Damage`) (`KismetMathLibrary.RandomFloatInRange` 0.9 1.1)))
  (bind _returnvalue_2 (* (`self.Damage`) (`KismetMathLibrary.RandomFloatInRange` 0.5 0.7)))
  (bind _returnvalue_3 (* (`self.Damage`) (`KismetMathLibrary.RandomFloatInRange` 1.2 1.4)))
  (if (!= OtherActor (`self.ProjectileOwner`))
    (set `self.OverlapActor` OtherActor)
    (`/Engine/EditorBlueprintResources/ActorMacros.Switch Has Authority`
      (:`Authority`
        (bind _asmy_insane_party_character (cast `/Game/MyInsanePartyCharacter` (`self.ProjectileOwner`))
          (:`then`
            (bind _asmy_insane_party_character_2 (cast `/Game/MyInsanePartyCharacter` (`self.OverlapActor`))
              (:`then`
                (bind _returnvalue_4 (`AbilitySystemBlueprintLibrary.GetAbilitySystemComponent` _asmy_insane_party_character_2))
                (if (`KismetSystemLibrary.IsValid` _returnvalue_4)
                  (bind (_outhits _returnvalue_5) (`KismetSystemLibrary.SphereTraceMultiForObjects` :`Start` (`self.K2_GetActorLocation`) :`End` (`self.K2_GetActorLocation` (`self.OverlapActor`)) :`Radius` 15.0 :`ObjectTypes` (`|MakeArray` "ObjectTypeQuery3" :!type "EObjectTypeQuery Enum") :`bTraceComplex` true :`TraceColor` (struct :`R` 0.456411 :`G` 0.212231 :`B` 1.0 :`A` 1.0) :`TraceHitColor` (struct :`R` 0.456411 :`G` 0.212231 :`B` 1.0 :`A` 1.0) :`DrawTime` 1.0))
                  (if _returnvalue_5
                    (for _array_element _outhits
                      (bind (_bblockinghit _binitialoverlap _time _distance _location _impactpoint _normal _impactnormal _physmat _hitactor _hitcomponent _hitbonename) (`GameplayStatics.BreakHitResult` _array_element))
                      (if (and (== _hitactor _asmy_insane_party_character_2) (!= _hitbonename "None"))
                        (break)))
                    (bind _output_get (set `self.HitResult` _array_element))
                    (bind _returnvalue_6 (`AbilitySystemComponent.MakeEffectContext` (`AbilitySystemBlueprintLibrary.GetAbilitySystemComponent` _asmy_insane_party_character)))
                    (`AbilitySystemBlueprintLibrary.EffectContextAddHitResult` _returnvalue_6 _output_get)
                    (switch `name` _hitbonename
                      (:`Default`
                        (`KismetSystemLibrary.PrintString` (`KismetStringLibrary.Conv_DoubleToString` _returnvalue_2))
                        (bind _returnvalue_7 (`AbilitySystemComponent.MakeOutgoingSpec` _returnvalue_4 "/Game/Blueprints/GameplayAbilitySystem/GameplayEffects/GE_Damaging.GE_Damaging_C" 0.0 _returnvalue_6))
                        (bind _returnvalue_8 (`AbilitySystemBlueprintLibrary.AssignTagSetByCallerMagnitude` _returnvalue_7 (struct :`TagName` "GameplayEffect.Damage") _returnvalue_2))
                        (`AbilitySystemComponent.BP_ApplyGameplayEffectSpecToSelf` _returnvalue_4 _returnvalue_8))
                      (:`head`
                        (`KismetSystemLibrary.PrintString` (`KismetStringLibrary.Conv_DoubleToString` _returnvalue_3) :!label _label)
                        (bind _returnvalue_9 (`AbilitySystemBlueprintLibrary.AssignTagSetByCallerMagnitude` _returnvalue_7 (struct :`TagName` "GameplayEffect.Damage") _returnvalue_3))
                        (`AbilitySystemComponent.BP_ApplyGameplayEffectSpecToSelf` _returnvalue_4 _returnvalue_9))
                      (:`neck_01`
                        (goto _label))
                      (:`neck_02`
                        (goto _label))
                      (:`pelvis`
                        (`KismetSystemLibrary.PrintString` (`KismetStringLibrary.Conv_DoubleToString` _returnvalue) :!label _label_2)
                        (bind _returnvalue_10 (`AbilitySystemBlueprintLibrary.AssignTagSetByCallerMagnitude` _returnvalue_7 (struct :`TagName` "GameplayEffect.Damage") _returnvalue))
                        (`AbilitySystemComponent.BP_ApplyGameplayEffectSpecToSelf` _returnvalue_4 _returnvalue_10))
                      (:`spine_01`
                        (goto _label_2))
                      (:`spine_02`
                        (goto _label_2))
                      (:`spine_03`
                        (goto _label_2))
                      (:`spine_04`
                        (goto _label_2))
                      (:`spine_05`
                        (goto _label_2))
                      (:`upperarm_l`
                        (goto _label_2))
                      (:`upperarm_r`
                        (goto _label_2))
                      (:`clavicle_l`
                        (goto _label_2))
                      (:`clavicle_out_l`
                        (goto _label_2))
                      (:`clavicle_scap_l`
                        (goto _label_2))
                      (:`clavicle_out_r`
                        (goto _label_2))
                      (:`clavicle_pec_l`
                        (goto _label_2))
                      (:`clavicle_pec_r`
                        (goto _label_2))
                      (:`clavicle_r`
                        (goto _label_2)))
                    (`self.MC_PlayAnim` _asmy_insane_party_character_2)
                    (`self.K2_DestroyActor`))))
              (:`CastFailed`
                (`self.K2_DestroyActor` :!label _label_3))))
          (:`CastFailed`
            (goto _label_3))))
      (:`Remote`
        (goto _label_3)))))

(event `MC_PlayAnim`
  (params (Target :type "Character Object Reference"))
  (`Character.PlayAnimMontage` Target "/Game/NewAnimMontage.NewAnimMontage" 0.03 "None"))

(fn `UserConstructionScript`)