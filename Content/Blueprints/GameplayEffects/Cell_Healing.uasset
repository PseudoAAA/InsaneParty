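; Healing cell actor, by its name, that applies a configurable Gameplay Effect to actors inside its box trigger.
; Overlapping actors with an Ability System Component receive the effect on entry and lose all its stacks on exit.
; The first valid overlap starts a one-shot timer through DoOnce, which removes the cell seconds later by setting a near-zero lifespan.
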(event `self.Box.OnComponentBeginOverlap`
  (params (OverlappedComponent :type "PrimitiveComponent Object Reference") (OtherActor :type "Actor Object Reference") (OtherComp :type "PrimitiveComponent Object Reference") (OtherBodyIndex :type Integer) (bFromSweep :type Boolean) (SweepResult :type "HitResult Structure (by ref)"))
  (bind _returnvalue (`AbilitySystemBlueprintLibrary.GetAbilitySystemComponent` OtherActor))
  (`/Engine/EditorBlueprintResources/StandardMacros.IsValid` _returnvalue
    (:`Is Valid`
      (`AbilitySystemComponent.BP_ApplyGameplayEffectToSelf` :`self` _returnvalue :`GameplayEffectClass` (`self.GameplayEffectToApply`))
      (`/Engine/EditorBlueprintResources/StandardMacros.DoOnce` false
        (:`Completed`
          (`KismetSystemLibrary.K2_SetTimerDelegate` (delegate `RemoveCell`) 5.0)
          (`KismetSystemLibrary.PrintString` "Timer has been started"))))))

(event `RemoveCell`
  (`self.SetLifeSpan` 0.0001))

(event `self.Box.OnComponentEndOverlap`
  (params (OverlappedComponent :type "PrimitiveComponent Object Reference") (OtherActor :type "Actor Object Reference") (OtherComp :type "PrimitiveComponent Object Reference") (OtherBodyIndex :type Integer))
  (bind _returnvalue (`AbilitySystemBlueprintLibrary.GetAbilitySystemComponent` OtherActor))
  (`/Engine/EditorBlueprintResources/StandardMacros.IsValid` _returnvalue
    (:`Is Valid`
      (`AbilitySystemComponent.RemoveActiveGameplayEffectBySourceEffect` _returnvalue (`self.GameplayEffectToApply`) null -1))))

(fn `UserConstructionScript`)