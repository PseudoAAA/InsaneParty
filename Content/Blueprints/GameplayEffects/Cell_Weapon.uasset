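; Cell_Weapon is a weapon pickup actor that uses the Gameplay Ability System.
; When an actor with an ability system component overlaps its Box, it grants that actor GA_PickupWeapon and immediately tries to activate it.
; If activation succeeds, it also grants GA_EquipWeapon and removes itself through a near-zero lifespan.
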(event `self.Box.OnComponentBeginOverlap`
  (params (OverlappedComponent :type "PrimitiveComponent Object Reference") (OtherActor :type "Actor Object Reference") (OtherComp :type "PrimitiveComponent Object Reference") (OtherBodyIndex :type Integer) (bFromSweep :type Boolean) (SweepResult :type "HitResult Structure (by ref)"))
  (bind _returnvalue (`AbilitySystemBlueprintLibrary.GetAbilitySystemComponent` OtherActor))
  (`/Engine/EditorBlueprintResources/StandardMacros.IsValid` _returnvalue
    (:`Is Valid`
      (bind _returnvalue_2 (`AbilitySystemComponent.K2_GiveAbility` _returnvalue "/Game/Blueprints/GameplayEffects/GA_PickupWeapon.GA_PickupWeapon_C" 0 -1))
      (bind _returnvalue_3 (`AbilitySystemComponent.TryActivateAbility` _returnvalue _returnvalue_2 true))
      (if _returnvalue_3
        (`AbilitySystemComponent.K2_GiveAbility` _returnvalue "/Game/Blueprints/GameplayEffects/GA_EquipWeapon.GA_EquipWeapon_C" 0 -1)
        (`self.SetLifeSpan` 0.0001)))))

(fn `UserConstructionScript`
  (`parent.UserConstructionScript`))