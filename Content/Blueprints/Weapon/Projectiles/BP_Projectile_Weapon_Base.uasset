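; Base weapon projectile that damages characters through GAS and leaves bullet holes on static surfaces, with lifespan set by range over speed.
; On a server-side capsule overlap, a capsule trace finds the hit bone, scaling GE_Damaging's SetByCaller damage for head/neck, torso/upper arms or other areas.
; Character hits also increment the victim's hit counter and trigger a montage.
; Otherwise a line trace locates static geometry for a decal spawned only on remotes.
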(event `self.ReceiveBeginPlay`
  (`/Engine/EditorBlueprintResources/ActorMacros.Switch Has Authority`
    (:`Authority`
      (`SceneComponent.SetVisibility` (`self.Sphere`) false false))
    (:`Remote`
      _))
  (set `self.ProjectileOwner` (`self.GetOwner`))
  (`self.SetLifeSpan` (/ (`self.Range`) (`self.InitialSpeed`))))

(event `self.Capsule.OnComponentBeginOverlap`
  (params (OverlappedComponent :type "PrimitiveComponent Object Reference") (OtherActor :type "Actor Object Reference") (OtherComp :type "PrimitiveComponent Object Reference") (OtherBodyIndex :type Integer) (bFromSweep :type Boolean) (SweepResult :type "HitResult Structure (by ref)"))
  (bind _sphere (`self.Sphere`))
  (bind _sphere_2 (`self.Sphere`))
  (bind _outspec (`self.OutSpec`))
  (bind _asc (`self.ASC`))
  (bind _returnvalue (`SceneComponent.K2_GetComponentLocation` _sphere))
  (bind _returnvalue_2 (`SceneComponent.K2_GetComponentLocation` _sphere_2))
  (bind _returnvalue_3 (`KismetMathLibrary.Round` (* (`self.Damage`) 0.9)))
  (bind _returnvalue_4 (`KismetMathLibrary.Round` (* (`self.Damage`) 1.2)))
  (bind _returnvalue_5 (`KismetMathLibrary.Round` (* (`self.Damage`) 0.6)))
  (if (!= OtherActor (`self.ProjectileOwner`))
    (set `self.OverlapActor` OtherActor)
    (`/Engine/EditorBlueprintResources/ActorMacros.Switch Has Authority`
      (:`Authority`
        (bind _asinsane_party_character (cast `InsanePartyCharacter` (`self.ProjectileOwner`))
          (:`then`
            (bind _asinsane_party_character_2 (cast `InsanePartyCharacter` (`self.OverlapActor`))
              (:`then`
                (bind _returnvalue_6 (`AbilitySystemBlueprintLibrary.GetAbilitySystemComponent` _asinsane_party_character_2))
                (set `self.ASC` _returnvalue_6)
                (set `self.As Insane Party Character` _asinsane_party_character_2)
                (if (`KismetSystemLibrary.IsValid` _returnvalue_6)
                  (bind _returnvalue_7 (`AbilitySystemComponent.MakeEffectContext` (`AbilitySystemBlueprintLibrary.GetAbilitySystemComponent` _asinsane_party_character)))
                  (set `self.OutSpec` (`AbilitySystemComponent.MakeOutgoingSpec` _returnvalue_6 "/Game/Blueprints/GameplayAbilitySystem/GameplayEffects/GE_Damaging.GE_Damaging_C" 0.0 _returnvalue_7))
                  (bind (_outhits _returnvalue_8) (`KismetSystemLibrary.CapsuleTraceMultiForObjects` _returnvalue (+ _returnvalue (* (`SceneComponent.GetUpVector` _sphere) 150.0)) 15.0 5.0 (`|MakeArray` "ObjectTypeQuery3" :!type "EObjectTypeQuery Enum") true))
                  (if _returnvalue_8
                    (for _array_element _outhits
                      (bind (_bblockinghit _binitialoverlap _time _distance _location _impactpoint _normal _impactnormal _physmat _hitactor _hitcomponent _hitbonename) (`GameplayStatics.BreakHitResult` _array_element))
                      (if (and (== _hitactor (`self.OverlapActor`)) (!= _hitbonename "None"))
                        (break)))
                    (bind _output_get (set `self.HitResult` _array_element))
                    (`AbilitySystemBlueprintLibrary.EffectContextAddHitResult` _returnvalue_7 _output_get)
                    ;[0.3073 0.1905 0.1905] I THINK IS A BAD REALIZATION
                    (switch `name` _hitbonename
                      (:`Default`
                        (`KismetSystemLibrary.PrintString` (`KismetStringLibrary.Conv_IntToString` _returnvalue_5))
                        (bind _returnvalue_9 (`AbilitySystemBlueprintLibrary.AssignTagSetByCallerMagnitude` _outspec (struct :`TagName` "GameplayEffect.Damage") (`KismetMathLibrary.Conv_IntToDouble` _returnvalue_5)))
                        (`AbilitySystemComponent.BP_ApplyGameplayEffectSpecToSelf` _asc _returnvalue_9))
                      (:`head`
                        (`KismetSystemLibrary.PrintString` (`KismetStringLibrary.Conv_IntToString` _returnvalue_4) :!label _label)
                        (bind _returnvalue_10 (`AbilitySystemBlueprintLibrary.AssignTagSetByCallerMagnitude` _outspec (struct :`TagName` "GameplayEffect.Damage") (`KismetMathLibrary.Conv_IntToDouble` _returnvalue_4)))
                        (`AbilitySystemComponent.BP_ApplyGameplayEffectSpecToSelf` _asc _returnvalue_10))
                      (:`neck_01`
                        (goto _label))
                      (:`neck_02`
                        (goto _label))
                      (:`pelvis`
                        (`KismetSystemLibrary.PrintString` (`KismetStringLibrary.Conv_IntToString` _returnvalue_3) :!label _label_2)
                        (bind _returnvalue_11 (`AbilitySystemBlueprintLibrary.AssignTagSetByCallerMagnitude` _outspec (struct :`TagName` "GameplayEffect.Damage") (`KismetMathLibrary.Conv_IntToDouble` _returnvalue_3)))
                        (`AbilitySystemComponent.BP_ApplyGameplayEffectSpecToSelf` _asc _returnvalue_11))
                      (:`spine_01`
                        (goto _label_2))
                      (:`spine_02`
                        (goto _label_2))
                      (:`spine_03`
                        (goto _label_2))
                      (:`spine_04`
                        (goto _label_2))
                      (:`spine_05`
                        (goto _label_2))
                      (:`upperarm_l`
                        (goto _label_2))
                      (:`upperarm_r`
                        (goto _label_2))
                      (:`clavicle_l`
                        (goto _label_2))
                      (:`clavicle_out_l`
                        (goto _label_2))
                      (:`clavicle_scap_l`
                        (goto _label_2))
                      (:`clavicle_out_r`
                        (goto _label_2))
                      (:`clavicle_pec_l`
                        (goto _label_2))
                      (:`clavicle_pec_r`
                        (goto _label_2))
                      (:`clavicle_r`
                        (goto _label_2)))
                    (bind _asbp_insane_party_character (cast `/Game/BP_InsanePartyCharacter` (`self.As Insane Party Character`)))
                    (set `/Game/BP_InsanePartyCharacter.CountHits` (+ (`/Game/BP_InsanePartyCharacter.CountHits` _asbp_insane_party_character) 1.0) _asbp_insane_party_character)
                    (`self.CustomEvent_1` (`self.As Insane Party Character`))
                    (`self.K2_DestroyActor`)
                    (else
                      (bind (_outhit _returnvalue_12) (`KismetSystemLibrary.LineTraceSingleForObjects` :`Start` _returnvalue_2 :`End` (+ _returnvalue_2 (* (`SceneComponent.GetUpVector` _sphere_2) 500.0)) :`ObjectTypes` (`|MakeArray` "ObjectTypeQuery1" :!type "EObjectTypeQuery Enum") :`bTraceComplex` true :`DrawTime` 2.0 :!label _label_3))
                      (if _returnvalue_12
                        (bind (_bblockinghit_2 _binitialoverlap_2 _time_2 _distance_2 _location_2 _impactpoint_2 _normal_2 _impactnormal_2 _physmat_2 _hitactor_2 _hitcomponent_2 _hitbonename_2) (`GameplayStatics.BreakHitResult` _outhit))
                        (`self.CustomEvent` _hitcomponent_2 _hitbonename_2 _location_2 (`KismetMathLibrary.Conv_VectorToRotator` _impactnormal_2))
                        (`self.K2_DestroyActor`))))
                  (else
                    (goto _label_3))))
              (:`CastFailed`
                (goto _label_3))))
          (:`CastFailed`
            (goto _label_3))))
      (:`Remote`
        (`self.K2_DestroyActor`)))))

(event `CustomEvent`
  (params (AttachToComponent :type "SceneComponent Object Reference") (AttachPointName :type Name) (Location :type "Vector Structure") (Rotation :type "Rotator Structure"))
  (`/Engine/EditorBlueprintResources/ActorMacros.Switch Has Authority`
    (:`Remote`
      (bind _returnvalue (`GameplayStatics.SpawnDecalAttached` "/Game/Blueprints/Weapon/Rifle/M_RifleBulletHole.M_RifleBulletHole" (10.0 10.0 10.0) AttachToComponent AttachPointName Location Rotation "KeepWorldPosition" 30.0))
      (bind _asdecal_component (cast `DecalComponent` _returnvalue))
      (`DecalComponent.SetFadeScreenSize` _asdecal_component 0.0))))

(event `CustomEvent_1`
  (params (Target :type "Character Object Reference"))
  (`Character.PlayAnimMontage` Target "/Game/NewAnimMontage.NewAnimMontage" 0.03 "None"))

(fn `UserConstructionScript`)