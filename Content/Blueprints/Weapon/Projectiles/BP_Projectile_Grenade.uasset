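; Grenade projectile that explodes on a timer set to its lifespan, playing a sound and damaging party characters in range.
; The explosion gathers overlapping actors, filters them by line of sight via player controller 0 from the grenade's location, and shakes hit characters' cameras.
; Living victims receive GAS damage through a SetByCaller effect applied by their own ability system.
; The first collision overlap switches collision responses to overlap.
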(event `self.ReceiveBeginPlay`
  (`parent.ReceiveBeginPlay`)
  (`KismetSystemLibrary.K2_SetTimerDelegate` (delegate `self.Explode`) (`self.GetLifeSpan`)))

(event `self.Explode`
  (`self.MC_SpawnSound` (`self.Explosion Sound`) (`SceneComponent.K2_GetComponentLocation` (`self.ProjectileMesh`)))
  (`self.SR_ExplodeEvent`))

(event `self.ProjectileCollision.OnComponentBeginOverlap`
  (params (OverlappedComponent :type "PrimitiveComponent Object Reference") (OtherActor :type "Actor Object Reference") (OtherComp :type "PrimitiveComponent Object Reference") (OtherBodyIndex :type Integer) (bFromSweep :type Boolean) (SweepResult :type "HitResult Structure (by ref)"))
  (`/Engine/EditorBlueprintResources/StandardMacros.DoOnce` false
    (:`Completed`
      (`PrimitiveComponent.SetCollisionResponseToChannel` (`self.ProjectileMesh`) "ECC_Pawn" "ECR_Overlap")
      (`PrimitiveComponent.SetCollisionResponseToAllChannels` (`self.ProjectileCollision`) "ECR_Overlap"))))

(event `self.SR_ExplodeEvent`
  (for _array_element (`PrimitiveComponent.GetOverlappingActors` (`self.ExplosionCollision`) null)
    (if (`Controller.LineOfSightTo` (`GameplayStatics.GetPlayerController` 0) _array_element (`SceneComponent.K2_GetComponentLocation` (`self.RootComponent`)) false)
      (`KismetArrayLibrary.Array_AddUnique` (`self.HittedActors`) _array_element)))
  (for _array_element_2 (`self.HittedActors`)
    (bind _asbp_insane_party_character (cast `/Game/BP_InsanePartyCharacter` _array_element_2))
    (`/Game/BP_InsanePartyCharacter.GrenadeCameraShake` _asbp_insane_party_character)
    (bind _returnvalue (`InsanePartyCharacterBase.IsAlive` _asbp_insane_party_character))
    (if _returnvalue
      (bind _returnvalue_2 (`AbilitySystemBlueprintLibrary.GetAbilitySystemComponent` _asbp_insane_party_character))
      (bind _returnvalue_3 (`AbilitySystemBlueprintLibrary.AssignTagSetByCallerMagnitude` (`AbilitySystemComponent.MakeOutgoingSpec` _returnvalue_2 "/Game/Blueprints/GameplayAbilitySystem/GameplayEffects/GE_Damaging.GE_Damaging_C" 0.0 (`AbilitySystemComponent.MakeEffectContext` _returnvalue_2)) (struct :`TagName` "GameplayEffect.Damage") 50.0))
      (`AbilitySystemComponent.BP_ApplyGameplayEffectSpecToSelf` _returnvalue_2 _returnvalue_3))))

(fn `UserConstructionScript`
  (`parent.UserConstructionScript`))