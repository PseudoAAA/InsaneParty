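; BP_Pistol_Weapon is a pistol weapon pickup that goes into the interacting player's inventory.
; On Interact it casts the actor to the party character, gets the inventory system component from its player state and checks that the weapon is unique.
; A unique weapon is added with its data asset and magazine info, then the pickup removes itself through a very short lifespan.
; Otherwise it only prints a failure message.
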(event `InteractInterface.Interact`
  (params (AnActor :type "Actor Object Reference"))
  (bind _weapondata (`self.WeaponData`))
  (bind _asinsane_party_character_base (cast `InsanePartyCharacterBase` AnActor))
  (bind _asmy_insane_player_state (cast `/Game/MyInsanePlayerState` (`Pawn.PlayerState` _asinsane_party_character_base)))
  (bind _returnvalue (`InsanePlayerState.GetInventorySystemComponent` _asmy_insane_player_state))
  (`/Engine/EditorBlueprintResources/StandardMacros.IsValid` _returnvalue
    (:`Is Valid`
      (if (`InsaneInventorySystemComponent.IsUniqueWeapon` _returnvalue _weapondata)
        (`InsaneInventorySystemComponent.AddWeaponToInventory` _returnvalue _weapondata (make `WeaponData` _weapondata (`self.MagazineInfo`)))
        (`self.SetLifeSpan` 0.01)
        (else
          (`KismetSystemLibrary.PrintString` "Fail adding"))))))

(fn `UserConstructionScript`)