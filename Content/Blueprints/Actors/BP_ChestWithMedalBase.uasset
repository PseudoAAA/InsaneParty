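; BP_ChestWithMedalBase is a chest actor that grants keys on interaction and damages party characters that touch its box.
; Interact applies GE_AddKeys through the Ability System Component of the interacting player's PlayerState.
; Box overlap applies GE_Damaging to living characters, passing a fixed damage magnitude via SetByCaller.
; Despite the name, no medal is awarded; a medal-count check sits unconnected.
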(event `InteractInterface.Interact`
  (params (AnActor :type "Actor Object Reference"))
  (bind _asbp_insane_party_character (cast `/Game/BP_InsanePartyCharacter` AnActor))
  (bind _asmy_insane_player_state (cast `/Game/MyInsanePlayerState` (`Pawn.PlayerState` _asbp_insane_party_character)))
  (bind _returnvalue (`AbilitySystemBlueprintLibrary.GetAbilitySystemComponent` _asmy_insane_player_state))
  (`AbilitySystemComponent.BP_ApplyGameplayEffectToSelf` _returnvalue "/Game/Blueprints/GameplayAbilitySystem/GameplayEffects/GE_AddKeys.GE_AddKeys_C" 1.0 (`AbilitySystemComponent.MakeEffectContext` _returnvalue)))

(event `self.Box.OnComponentBeginOverlap`
  (params (OverlappedComponent :type "PrimitiveComponent Object Reference") (OtherActor :type "Actor Object Reference") (OtherComp :type "PrimitiveComponent Object Reference") (OtherBodyIndex :type Integer) (bFromSweep :type Boolean) (SweepResult :type "HitResult Structure (by ref)"))
  (bind _asbp_insane_party_character (cast `/Game/BP_InsanePartyCharacter` OtherActor))
  (bind _returnvalue (`InsanePartyCharacterBase.IsAlive` _asbp_insane_party_character))
  (if _returnvalue
    (bind _returnvalue_2 (`AbilitySystemBlueprintLibrary.GetAbilitySystemComponent` _asbp_insane_party_character))
    (bind _returnvalue_3 (`AbilitySystemBlueprintLibrary.AssignTagSetByCallerMagnitude` (`AbilitySystemComponent.MakeOutgoingSpec` _returnvalue_2 "/Game/Blueprints/GameplayAbilitySystem/GameplayEffects/GE_Damaging.GE_Damaging_C" 0.0 (`AbilitySystemComponent.MakeEffectContext` _returnvalue_2)) (struct :`TagName` "GameplayEffect.Damage") 100.0))
    (`AbilitySystemComponent.BP_ApplyGameplayEffectSpecToSelf` _returnvalue_2 _returnvalue_3)))

(fn `NewFunction`
  (params (Object :type "Object Object Reference")))

(fn `UserConstructionScript`)