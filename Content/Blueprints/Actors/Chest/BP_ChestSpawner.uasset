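; BP_ChestSpawner is an actor that spawns a BP_ChestWithMedals at its own location and rotation.
; Tick feeds a random Delay of a few seconds, which acts as a repeating check that no such chest exists in the level.
; After a spawn, the CanSpawn flag blocks that spawner for a two-minute cooldown.
; The class-wide search means any existing chest, whichever spawner made it, suppresses new spawns.
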(event `self.ReceiveTick`
  (params (DeltaSeconds :type "Float (single-precision)"))
  (`KismetSystemLibrary.Delay` (`KismetMathLibrary.RandomFloatInRange` 1.0 10.0))
  (if (`self.CanSpawn`)
    (bind _outactors (`GameplayStatics.GetAllActorsOfClass` "/Game/Blueprints/Actors/Chest/BP_ChestWithMedals.BP_ChestWithMedals_C"))
    (if (not (> (`KismetArrayLibrary.Array_Length` _outactors) 0))
      (`|SpawnActorFromClass` "/Game/Blueprints/Actors/Chest/BP_ChestWithMedals.BP_ChestWithMedals_C" (`KismetMathLibrary.MakeTransform` (`self.K2_GetActorLocation`) (`self.K2_GetActorRotation`)) "Undefined" "MultiplyWithRoot" null null)
      (set `self.CanSpawn` false)
      (`KismetSystemLibrary.Delay` 120.0)
      (set `self.CanSpawn` true))))

(fn `UserConstructionScript`)