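; Chest actor that a living BP_InsanePartyCharacter opens through GAS, gated on a positive attribute (likely keys).
; Each valid Interact applies GE_DecreaseKeys before a DoOnce, which then plays the chest sound and a lid-rotation timeline.
; When the timeline finishes, it grants the configurable effect (presumably medals) with a set-by-caller magnitude, then destroys itself after a short delay.
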(event `InteractInterface.Interact`
  (params (AnActor :type "Actor Object Reference"))
  (bind _asbp_insane_party_character (cast `/Game/BP_InsanePartyCharacter` AnActor))
  (bind _returnvalue (`InsanePartyCharacterBase.IsAlive` _asbp_insane_party_character))
  (bind _returnvalue_2 (`AbilitySystemBlueprintLibrary.GetAbilitySystemComponent` _asbp_insane_party_character))
  (if (and _returnvalue (> (`.ReturnValue` (`AbilitySystemBlueprintLibrary.GetFloatAttributeFromAbilitySystemComponent` _returnvalue_2 (struct :`AttributeName` "Keys" :`Attribute` "/Script/InsaneParty.InsaneAttributeSet:Keys" :`AttributeOwner` "/Script/CoreUObject.Class'/Script/InsaneParty.InsaneAttributeSet'"))) 0.0))
    (bind _returnvalue_3 (`AbilitySystemComponent.MakeEffectContext` _returnvalue_2))
    (`AbilitySystemComponent.BP_ApplyGameplayEffectToSelf` _returnvalue_2 "/Game/Blueprints/GameplayAbilitySystem/GameplayEffects/GE_DecreaseKeys.GE_DecreaseKeys_C" 0.0 _returnvalue_3)
    (`/Engine/EditorBlueprintResources/StandardMacros.DoOnce` false
      (:`Completed`
        (`self.CustomEvent`)
        (bind (_direction _newtrack_0) (`Timeline|Timeline` :!via `PlayFromStart`)
          (:`Update`
            (`SceneComponent.K2_SetRelativeRotation` (`self.SM_Chest_Top`) (`KismetMathLibrary.MakeRotator` _newtrack_0) false false))
          (:`Finished`
            (bind _returnvalue_4 (`AbilitySystemBlueprintLibrary.AssignTagSetByCallerMagnitude` (`AbilitySystemComponent.MakeOutgoingSpec` _returnvalue_2 (`self.GameplayEffectToApply`) 0.0 _returnvalue_3) (`self.Effect Tag`) (`self.Magnitude`)))
            (`AbilitySystemComponent.BP_ApplyGameplayEffectSpecToSelf` _returnvalue_2 _returnvalue_4)
            (`KismetSystemLibrary.Delay` 1.0)
            (`self.K2_DestroyActor`)))))))

(event `CustomEvent`
  (`GameplayStatics.SpawnSoundAtLocation` "/Game/Blueprints/Actors/Chest/ChestSound.ChestSound" (`self.K2_GetActorLocation`) (struct) 1.0 1.0 0.0 "/Game/Blueprints/Actors/Chest/SA_Base.SA_Base" null))

(fn `UserConstructionScript`)