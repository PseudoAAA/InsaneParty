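; Base test actor that applies a configurable gameplay effect to player characters entering its box trigger.
; On overlap by a living BP_InsanePartyCharacter, it builds an outgoing spec of GameplayEffectToApply from that character's ability system.
; It sets a set-by-caller magnitude from EffectTag and Magnitude, then applies the spec to that same character.
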(event `self.Box.OnComponentBeginOverlap`
  (params (OverlappedComponent :type "PrimitiveComponent Object Reference") (OtherActor :type "Actor Object Reference") (OtherComp :type "PrimitiveComponent Object Reference") (OtherBodyIndex :type Integer) (bFromSweep :type Boolean) (SweepResult :type "HitResult Structure (by ref)"))
  (bind _asbp_insane_party_character (cast `/Game/BP_InsanePartyCharacter` OtherActor))
  (bind _returnvalue (`InsanePartyCharacterBase.IsAlive` _asbp_insane_party_character))
  (if _returnvalue
    (bind _returnvalue_2 (`AbilitySystemBlueprintLibrary.GetAbilitySystemComponent` _asbp_insane_party_character))
    (bind _returnvalue_3 (`AbilitySystemBlueprintLibrary.AssignTagSetByCallerMagnitude` (`AbilitySystemComponent.MakeOutgoingSpec` _returnvalue_2 (`self.GameplayEffectToApply`) 0.0 (`AbilitySystemComponent.MakeEffectContext` _returnvalue_2)) (`self.Effect Tag`) (`self.Magnitude`)))
    (`AbilitySystemComponent.BP_ApplyGameplayEffectSpecToSelf` _returnvalue_2 _returnvalue_3)))

(fn `NewFunction`
  (params (Object :type "Object Object Reference")))

(fn `UserConstructionScript`)