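; GA_UnequipWeapon is a gameplay ability that moves the character's weapon from its equipped state back to the rifle socket.
; On successful commit, it messages the avatar, finds the first attached BP_WeaponBase actor and snaps it to the mesh's rifle_socket.
; It then removes effects granting the Weapon.Equipped tag and ends.
; Ending grants GA_EquipWeapon to the avatar's ability system, forming an equip/unequip toggle.
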(event `self.K2_ActivateAbility`
  (bind _returnvalue (`self.GetAvatarActorFromActorInfo`))
  (bind _returnvalue_2 (`self.K2_CommitAbility`))
  (if _returnvalue_2
    (message `/Game/Temp/Interfaces/BPI_WeaponWielder.UnequipWeapon` _returnvalue)
    (bind _asbp_third_person_character (cast `/Game/Blueprints/Characters/DefaultCharacter/BP_ThirdPersonCharacter` _returnvalue))
    (for _array_element (`Actor.GetAttachedActors` _asbp_third_person_character true false)
      (bind _returnvalue_3 (`KismetMathLibrary.ClassIsChildOf` (`GameplayStatics.GetObjectClass` _array_element) "/Game/Blueprints/Weapons/BP_WeaponBase.BP_WeaponBase_C"))
      (if _returnvalue_3
        (break)))
    (if _returnvalue_3
      (bind _asbp_weapon_base (cast `/Game/Blueprints/Weapons/BP_WeaponBase` _array_element))
      (`Actor.K2_AttachToComponent` _asbp_weapon_base (`Character.Mesh` _asbp_third_person_character) "rifle_socket" "SnapToTarget" "SnapToTarget" "KeepRelative" true)
      (`self.BP_RemoveGameplayEffectFromOwnerWithGrantedTags` (struct :`GameplayTags` (struct :`(TagName` "GameplayAbility.Weapon.Equipped"))))
      (`self.K2_EndAbility`))))

(event `self.K2_OnEndAbility`
  (params (bWasCancelled :type Boolean))
  (`AbilitySystemComponent.K2_GiveAbility` (`AbilitySystemBlueprintLibrary.GetAbilitySystemComponent` (`self.GetAvatarActorFromActorInfo`)) "/Game/Blueprints/GameplayAbilitySystem/GameplayAbilities/GA_EquipWeapon.GA_EquipWeapon_C" 0 -1))