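; GA_EquipWeapon is a Gameplay Ability that equips the third-person character's attached weapon.
; After committing, it messages the avatar, looks through its attached actors for a BP_WeaponBase, snaps that to the mesh's rifle equipped socket and messages it.
; It then removes effects granting the Unequipped tag and ends.
; On ending, it grants the unequip and shoot abilities to the avatar's ability system.
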(event `self.K2_ActivateAbility`
  (bind _returnvalue (`self.GetAvatarActorFromActorInfo`))
  (bind _returnvalue_2 (`self.K2_CommitAbility`))
  (if _returnvalue_2
    (message `/Game/Temp/Interfaces/BPI_WeaponWielder.EquipWeapon` _returnvalue)
    (bind _asbp_third_person_character (cast `/Game/Blueprints/Characters/DefaultCharacter/BP_ThirdPersonCharacter` _returnvalue))
    (for _array_element (`Actor.GetAttachedActors` _asbp_third_person_character true false)
      (if (== (`GameplayStatics.GetObjectClass` _array_element) "/Game/Blueprints/Weapons/BP_WeaponBase.BP_WeaponBase_C")
        _))
    (bind _asbp_weapon_base (cast `/Game/Blueprints/Weapons/BP_WeaponBase` _array_element))
    (`Actor.K2_AttachToComponent` _asbp_weapon_base (`Character.Mesh` _asbp_third_person_character) "rifle_equippedsocket" "SnapToTarget" "SnapToTarget" "KeepRelative" true)
    (message `/Game/Blueprints/Weapons/BPI_Weapon.EquipWeapon` _asbp_weapon_base)
    (`self.BP_RemoveGameplayEffectFromOwnerWithGrantedTags` (struct :`GameplayTags` (struct :`(TagName` "GameplayAbility.Weapon.Unequipped"))))
    (`self.K2_EndAbility`)))

(event `self.K2_OnEndAbility`
  (params (bWasCancelled :type Boolean))
  (bind _returnvalue (`AbilitySystemBlueprintLibrary.GetAbilitySystemComponent` (`self.GetAvatarActorFromActorInfo`)))
  (`AbilitySystemComponent.K2_GiveAbility` _returnvalue "/Game/Blueprints/GameplayAbilitySystem/GameplayAbilities/GA_UnequipWeapon.GA_UnequipWeapon_C" 0 -1)
  (`AbilitySystemComponent.K2_GiveAbility` _returnvalue "/Game/Blueprints/GameplayAbilitySystem/GameplayAbilities/GA_Shoot.GA_Shoot_C" 5 -1))