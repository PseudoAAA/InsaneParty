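; GA_Shoot is a Gameplay Ability for shooting, with empty activation and end-ability events.
; Its ShootTrace function runs a debug-drawn multi sphere trace for Pawns along the avatar's forward vector, starting just ahead of it.
; Hit actors are added uniquely to HittedActors, which is returned and never cleared here.
; Nothing in this file calls ShootTrace or applies damage or effects.
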(event `self.K2_ActivateAbility`)

(event `self.K2_OnEndAbility`
  (params (bWasCancelled :type Boolean)))

(fn `ShootTrace`
  (returns (HittedActors :type "Array of Actor Object Reference"))
  (bind _returnvalue (`self.GetAvatarActorFromActorInfo`))
  (bind _returnvalue_2 (`Actor.K2_GetActorLocation` _returnvalue))
  (bind _returnvalue_3 (`Actor.GetActorForwardVector` _returnvalue))
  (bind _outhits (`KismetSystemLibrary.SphereTraceMultiForObjects` :`Start` (+ _returnvalue_2 (* _returnvalue_3 25.0)) :`End` (+ _returnvalue_2 (* _returnvalue_3 1000.0)) :`Radius` 5.0 :`ObjectTypes` (`|MakeArray` "ObjectTypeQuery3" :!type "EObjectTypeQuery Enum") :`DrawDebugType` "ForDuration" :`DrawTime` 1.0))
  (for _array_element _outhits
    (`KismetArrayLibrary.Array_AddUnique` (`self.HittedActors`) (`.HitActor` (`GameplayStatics.BreakHitResult` _array_element))))
  (return (`self.HittedActors`)))