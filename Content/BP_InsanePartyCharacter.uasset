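; Player character Blueprint for InsaneParty that handles a few inputs, weapon recoil and the local player's UI.
; Drop-weapon and reload keys activate Gameplay Ability System abilities by tag through the PlayerState's ability system component.
; IMPRecoil plays a timeline that adds randomized pitch and yaw input, while the plain Recoil event is empty.
; Shooting, aiming, fire-mode, slot-switching and trace-debug logic is disconnected; a debug key prints hit count.
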(event Custom|Recoil
  (params (RecoilAmplitude :type Float%20%28single-precision%29) (SidewaysRecoil :type Float%20%28single-precision%29) (Min :type Float%20%28single-precision%29) (Max :type Float%20%28single-precision%29)))

(event EventBeginPlay
  (if (Pawn|IsLocallyControlled)
    (bind _returnvalue (UserInterface|CreateWidget "/Game/Blueprints/UI/WBP_PlayerUI.WBP_PlayerUI_C"))
    (UserInterface|Viewport|AddtoViewport _returnvalue 0)))

(event EventIMPRecoil
  (params (RecoilAmplitude :type Float%20%28single-precision%29) (SidewaysRecoilAmplitude :type Float%20%28single-precision%29) (Min :type Float%20%28single-precision%29) (Max :type Float%20%28single-precision%29))
  (bind _recoil (Timeline|Timeline PlayFromStart)
    (:Update
      (Pawn|Input|AddControllerPitchInput (* (* (* _recoil RecoilAmplitude) (Math|Random|RandomFloatinRange Min Max)) (Variables|Default|GetLookUpRate) (Utilities|Time|GetWorldDeltaSeconds)))
      (Pawn|Input|AddControllerYawInput (* (* (* (* (* _recoil RecoilAmplitude) (Math|Random|RandomFloatinRange Min Max)) SidewaysRecoilAmplitude) (Math|Random|RandomFloatinRange -1.0 1.0)) (Variables|Default|GetTurnRate) (Utilities|Time|GetWorldDeltaSeconds))))))

(event Input|KeyboardEvents|DebugKeyB
  (params (Key :type Key%20Structure :default "None") (ActionValue :type Input%20Action%20Value%20Structure)))

(event Input|KeyboardEvents|DebugKeyR
  (params (Key :type Key%20Structure :default "None") (ActionValue :type Input%20Action%20Value%20Structure))
  (:Pressed
    (bind _asmy_insane_player_state (Utilities|Casting|CastToMyInsanePlayerState (Variables|Default|GetPlayerState)))
    (Abilities|TryActivateAbilitiesbyTag (Ability|GetAbilitySystemComponent _asmy_insane_player_state) (GameplayTags|MakeGameplayTagContainerfromTag "(TagName=\"PlayerActions.Reload\")") true)))

(event Input|KeyboardEvents|DebugKey1
  (params (Key :type Key%20Structure :default "None") (ActionValue :type Input%20Action%20Value%20Structure)))

(event Input|KeyboardEvents|DebugKey3
  (params (Key :type Key%20Structure :default "None") (ActionValue :type Input%20Action%20Value%20Structure)))

(event Input|KeyboardEvents|DebugKey2
  (params (Key :type Key%20Structure :default "None") (ActionValue :type Input%20Action%20Value%20Structure)))

(event Input|KeyboardEvents|DebugKeyJ
  (params (Key :type Key%20Structure :default "None") (ActionValue :type Input%20Action%20Value%20Structure))
  (:Pressed
    (Development|PrintString (Utilities|String|ToString(Float) (Variables|Default|GetCountHits)))))

(event Input|KeyboardEvents|G
  (params (Key :type Key%20Structure :default "None"))
  (:Pressed
    (bind _asmy_insane_player_state (Utilities|Casting|CastToMyInsanePlayerState (Variables|Default|GetPlayerState)))
    (Abilities|TryActivateAbilitiesbyTag (Ability|GetAbilitySystemComponent _asmy_insane_player_state) (GameplayTags|MakeGameplayTagContainerfromTag "(TagName=\"Inventory.DropWeapon\")") true)))

(event Input|KeyboardEvents|5
  (params (Key :type Key%20Structure :default "None")))

(fn ConstructionScript)

(fn DebugTrace
  (bind _followcamera (Variables|Default|GetFollowCamera))
  (bind _returnvalue (Transformation|GetWorldLocation _followcamera))
  (bind (_outhit _returnvalue_2) (Collision|LineTraceForObjects _returnvalue (+ _returnvalue (* (Math|Vector|GetForwardVector _followcamera) 2e+03)) (Utilities|Array|MakeArray "ObjectTypeQuery1") true 0 "ForDuration"))
  (if _returnvalue_2
    (Development|PrintString (Utilities|GetDisplayName (.PhysMat (Collision|BreakHitResult _outhit))))
    (return)))